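; BP_PickUpMaster is a master Blueprint for pickup interactables whose mesh and physics depend on how the item enters the world.
; On BeginPlay, SetCraftableMesh switches on SpawnStatus and passes either the spawned or dropped item mesh to SetMesh.
; SetMesh checks the supplied mesh before applying it to DefaultMesh.
; Dropped items then enable physics simulation on DefaultMesh.
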(event `self.ReceiveBeginPlay`
  (`parent.ReceiveBeginPlay`)
  (`self.SetCraftableMesh`)
  (if (`|EnumEquality` (`self.SpawnStatus`) "NewEnumerator12")
    (`PrimitiveComponent.SetSimulatePhysics` (`self.DefaultMesh`) true)))

(fn `SetCraftableMesh`
  (switch `/Game/GameFiles/Interactables/Enums/E_CraftablesEnum` (`self.SpawnStatus`)
    (:`NewEnumerator8`
      (`self.SetMesh` (`self.SpawnedItemMesh`)))
    (:`NewEnumerator12`
      (`self.SetMesh` (`self.DroppedItemMesh`)))))

(fn `SetMesh`
  (params (ItemMesh :type "StaticMesh Object Reference"))
  (if (!= ItemMesh null)
    (`StaticMeshComponent.SetStaticMesh` (`self.DefaultMesh`) ItemMesh)))

(fn `UserConstructionScript`
  (`parent.UserConstructionScript`))