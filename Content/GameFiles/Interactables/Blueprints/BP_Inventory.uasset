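; Tabbed inventory that stores items in Useables, Armor, Quest and Readables slot arrays, and shows or hides its widget.
; AddItem routes items by type, fills a free stack or empty slot, recurses on overflow and returns any rest when full.
; Slot queries and removal work on tabs, with widget slots refreshed by index.
; Swap, merge, split and click functions are unfinished stubs.
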(event `self.ReceiveBeginPlay`
  (bind _currentinventoryslots (`self.CurrentInventorySlots`))
  (`self.InitialiseSlots`)
  (set `self.UseableItemSlots` _currentinventoryslots)
  (set `self.ArmorItemSlots` _currentinventoryslots)
  (set `self.QuestItemSlots` _currentinventoryslots)
  (set `self.ReadablesItemSlots` _currentinventoryslots))

(event `UpdateSlotAtIndex`
  (params (Index :type Integer))
  (`/Game/GameFiles/HUDs/InventoryHUD/InventorySlotHUDv1.UpdateSlot` (`|GetArrayItem` (`/Game/GameFiles/HUDs/InventoryHUD/InventoryHUDv2.SlotWidgets` (`self.InventoryWidget`)) Index)))

(event `UpdateCurrentInventoryTab`
  (params (CurrentInventoryTab :type "/Game/GameFiles/Interactables/Enums/E_InventoryTabEnum Enum" :default "NewEnumerator8"))
  (switch `/Game/GameFiles/Interactables/Enums/E_InventoryTabEnum` CurrentInventoryTab
    (:`NewEnumerator8`
      (set `self.CurrentInventorySlots` (`self.UseableItemSlots`)))
    (:`NewEnumerator10`
      (set `self.CurrentInventorySlots` (`self.ArmorItemSlots`)))
    (:`NewEnumerator0`
      (set `self.CurrentInventorySlots` (`self.QuestItemSlots`)))
    (:`NewEnumerator1`
      (set `self.CurrentInventorySlots` (`self.ReadablesItemSlots`)))))

(event `UpdateCurrentInventorySlots`
  (params (CurrentInventoryTab :type "/Game/GameFiles/Interactables/Enums/E_InventoryTabEnum Enum" :default "NewEnumerator8")))

(fn `AddItem`
  (params (ItemClass :type "/Game/GameFiles/Interactables/MasterBlueprints/BP_PickUpMaster Object Reference") (Amount :type Integer))
  (returns (`Success?` :type Boolean) (Rest :type Integer))
  (locals (LocalItemClass :type "/Game/GameFiles/Interactables/MasterBlueprints/BP_PickUpMaster Class Reference") (LocalAmount :type Integer) (FoundIndex :type Integer) (LocalItemReference :type "/Game/GameFiles/Interactables/MasterBlueprints/BP_PickUpMaster Object Reference") (ItemType :type "/Game/GameFiles/Interactables/Enums/E_ItemTypeEnum Enum"))
  (bind _returnvalue (`|EnumEquality` (`/Game/GameFiles/HUDs/InventoryHUD/InventoryHUDv2.CurrentInventoryTab` (`self.InventoryWidget`)) (`self.CurrentInventoryTab`)))
  (bind _output_get (set `local.LocalItemReference` ItemClass))
  (set `local.LocalAmount` Amount)
  (bind (_name _icon _itemtype _canbestacked_) (break `/Game/GameFiles/Interactables/Structs/S_ItemStruct` (`/Game/GameFiles/Interactables/MasterBlueprints/BP_PickUpMaster.ItemInfo` _output_get)))
  (set `local.ItemType` _itemtype)
  (if _canbestacked_
    (bind (_success_ _index) (`self.SearchFreeStack` (`local.LocalItemReference`) (`local.ItemType`)))
    (if _success_
      (bind _output_get_2 (set `local.FoundIndex` _index))
      (bind _returnvalue_2 (+ (`.Amount_7_22CE82A94F1C80878DBBB7851F6427BB` (break `/Game/GameFiles/Interactables/Structs/S_InventorySlots` (`|GetArrayItem` (stale _inventoryslot) _output_get_2))) (`local.LocalAmount`)))
      (if (> _returnvalue_2 (`self.MaxStackSize`))
        (set `local.LocalAmount` (- _returnvalue_2 (`self.MaxStackSize`)))
        (`self.SetItemInSlot` (`local.ItemType`) (`local.FoundIndex`) (`local.LocalItemReference`) (`self.MaxStackSize`))
        (if (`|EnumEquality` (`/Game/GameFiles/HUDs/InventoryHUD/InventoryHUDv2.CurrentInventoryTab` (`self.InventoryWidget`)) (`self.CurrentInventoryTab`))
          (`self.UpdateSlotAtIndex` (`local.FoundIndex`)))
        (bind (_success__2 _rest) (`self.AddItem` (`local.LocalItemReference`) (`local.LocalAmount`)))
        (return _success__2 _rest)
        (else
          (bind _inventoryslot (`self.GetItemSlot` (`local.ItemType`)))
          (`self.SetItemInSlot` (`local.ItemType`) (`local.FoundIndex`) (`local.LocalItemReference`) _returnvalue_2)
          (if (`|EnumEquality` (`/Game/GameFiles/HUDs/InventoryHUD/InventoryHUDv2.CurrentInventoryTab` (`self.InventoryWidget`)) (`self.CurrentInventoryTab`))
            (`self.UpdateSlotAtIndex` (`local.FoundIndex`)))
          (return true 0)))
      (else
        (bind (_success _index_2) (`self.SearchEmptySlot` (`local.ItemType`)))
        (if _success
          (set `local.FoundIndex` _index_2)
          (if (> (`local.LocalAmount`) (`self.MaxStackSize`))
            (`self.SetItemInSlot` (`local.ItemType`) (`local.FoundIndex`) (`local.LocalItemReference`) (`self.MaxStackSize`))
            (if _returnvalue
              (`self.UpdateSlotAtIndex` (`local.FoundIndex`)))
            (bind (_success__3 _rest_2) (`self.AddItem` (`local.LocalItemReference`) (- (`local.LocalAmount`) (`self.MaxStackSize`))))
            (return _success__3 _rest_2)
            (else
              (`self.SetItemInSlot` (`local.ItemType`) (`local.FoundIndex`) (`local.LocalItemReference`) (`local.LocalAmount`))
              (if _returnvalue
                (`self.UpdateSlotAtIndex` (`local.FoundIndex`)))
              (return true 0)))
          (else
            (return false (`local.LocalAmount`))))))
    (else
      (bind (_success_2 _index_3) (`self.SearchEmptySlot` (`local.ItemType`)))
      (if _success_2
        (set `local.FoundIndex` _index_3)
        (`self.SetItemInSlot` (`local.ItemType`) _index_3 (`local.LocalItemReference`) 1)
        (if (`|EnumEquality` (`/Game/GameFiles/HUDs/InventoryHUD/InventoryHUDv2.CurrentInventoryTab` (`self.InventoryWidget`)) (`self.CurrentInventoryTab`))
          (`self.UpdateSlotAtIndex` (`local.FoundIndex`)))
        (if (> (`local.LocalAmount`) 1)
          (bind (_success__4 _rest_3) (`self.AddItem` (`local.LocalItemReference`) (- (`local.LocalAmount`) 1)))
          (return _success__4 _rest_3)
          (else
            (return true 0)))
        (else
          (return false (`local.LocalAmount`)))))))

(fn `AddToIndex`
  (params (FromIndex :type Integer) (ToIndex :type Integer))
  (returns (`Success?` :type Boolean))
  (locals (LocalFrom :type Integer) (LocalTo :type Integer))
  (set `local.LocalFrom` FromIndex)
  (set `local.LocalTo` ToIndex)
  (if (not true)
    (return false)))

(fn `GetAmountAtIndex`
  (params (Index :type Integer))
  (returns (Amount :type Integer))
  (return (`.Amount_7_22CE82A94F1C80878DBBB7851F6427BB` (break `/Game/GameFiles/Interactables/Structs/S_InventorySlots` (`|GetArrayItem` (`self.GetItemTab` (`self.CurrentInventoryTab`)) Index)))))

(fn `GetItemInfoAtIndex`
  (params (Index :type Integer))
  (returns (`EmptySlot?` :type Boolean) (ItemInfo :type "/Game/GameFiles/Interactables/Structs/S_ItemStruct Structure") (AmountOfItems :type Integer))
  (bind (_iteminfo _itemmesh _amount) (break `/Game/GameFiles/Interactables/Structs/S_InventorySlots` (`|GetArrayItem` (`self.GetItemTab` (`/Game/GameFiles/HUDs/InventoryHUD/InventoryHUDv2.CurrentInventoryTab` (`self.InventoryWidget`))) Index)))
  (if (`KismetSystemLibrary.IsValid` _itemmesh)
    (return false _iteminfo _amount)
    (else
      (return true (struct) 0))))

(fn `GetItemSlot`
  (params (ItemType :type "/Game/GameFiles/Interactables/Enums/E_ItemTypeEnum Enum" :default "NewEnumerator8"))
  (returns (InventorySlot :type "Array of /Game/GameFiles/Interactables/Structs/S_InventorySlots Structure"))
  (switch `/Game/GameFiles/Interactables/Enums/E_ItemTypeEnum` ItemType
    (:`NewEnumerator8`
      _)
    (:`NewEnumerator12`
      _)
    (:`NewEnumerator0`
      (return (`self.ArmorItemSlots`)))
    (:`NewEnumerator1`
      (return (`self.ArmorItemSlots`)))
    (:`NewEnumerator2`
      (return (`self.ArmorItemSlots`)))
    (:`NewEnumerator3`
      (return (`self.ArmorItemSlots`)))
    (:`NewEnumerator4`
      (return (`self.ArmorItemSlots`)))
    (:`NewEnumerator5`
      (return (`self.ArmorItemSlots`)))
    (:`NewEnumerator6`
      (return (`self.ArmorItemSlots`)))
    (:`NewEnumerator7`
      (return (`self.ArmorItemSlots`)))
    (:`NewEnumerator9`
      (return (`self.QuestItemSlots`)))
    (:`NewEnumerator10`
      (return (`self.ReadablesItemSlots`))))
  (return (`self.UseableItemSlots`)))

(fn `GetItemTab`
  (params (ItemType :type "/Game/GameFiles/Interactables/Enums/E_InventoryTabEnum Enum" :default "NewEnumerator8"))
  (returns (InventorySlot :type "Array of /Game/GameFiles/Interactables/Structs/S_InventorySlots Structure"))
  (switch `/Game/GameFiles/Interactables/Enums/E_InventoryTabEnum` ItemType
    (:`NewEnumerator8`
      (return (`self.UseableItemSlots`)))
    (:`NewEnumerator10`
      (return (`self.ArmorItemSlots`)))
    (:`NewEnumerator0`
      (return (`self.QuestItemSlots`)))
    (:`NewEnumerator1`
      (return (`self.ReadablesItemSlots`)))))

(fn `HideInventory`
  (`Widget.SetVisibility` (`self.InventoryWidget`) "Hidden")
  (set `self.IsVisible?` false)
  (`Widget.SetIsEnabled` (`self.InventoryWidget`) false)
  (return))

(fn `InitialiseSlots`
  (`KismetArrayLibrary.Array_Resize` (`self.CurrentInventorySlots`) (`self.AmountOfSlots`)))

(fn `IsSlotEmpty?`
  (params (Index :type Integer))
  (returns (`Empty?` :type Boolean))
  (return (not (`KismetSystemLibrary.IsValid` (`.ItemMesh_17_ABCAB25E4B6C9235D6D6279073793DD2` (break `/Game/GameFiles/Interactables/Structs/S_InventorySlots` (`|GetArrayItem` (`self.GetItemTab` (`/Game/GameFiles/HUDs/InventoryHUD/InventoryHUDv2.CurrentInventoryTab` (`self.InventoryWidget`))) Index)))))))

(fn `OnSlotClicked`
  (params (Slot :type "/Game/GameFiles/HUDs/InventoryHUD/InventorySlotHUDv1 Object Reference")))

(fn `RemoveItemsAtIndex`
  (params (Index :type Integer) (Amount :type Integer))
  (returns (`Success?` :type Boolean))
  (locals (LocalIndex :type Integer) (LocalAmount :type Integer))
  (bind _inventoryslot (`self.GetItemTab` (`self.CurrentInventoryTab`)))
  (bind (_output_iteminfo _output_itemmesh _output_amount) (break `/Game/GameFiles/Interactables/Structs/S_InventorySlots` (`|GetArrayItem` _inventoryslot (`local.LocalIndex`))))
  (set `local.LocalIndex` Index)
  (set `local.LocalAmount` Amount)
  (if (and (not (`self.IsSlotEmpty?` (`local.LocalIndex`))) (> (`local.LocalAmount`) 0))
    (if (>= (`local.LocalAmount`) (`self.GetAmountAtIndex` (`local.LocalIndex`)))
      (`KismetArrayLibrary.Array_Set` (`self.GetItemTab` (`self.CurrentInventoryTab`)) (`local.LocalIndex`) (make `/Game/GameFiles/Interactables/Structs/S_InventorySlots` (struct :`ItemType` "NewEnumerator8")))
      (`self.UpdateSlotAtIndex` (`local.LocalIndex`))
      (return true)
      (else
        (`KismetArrayLibrary.Array_Set` _inventoryslot (`local.LocalIndex`) (make `/Game/GameFiles/Interactables/Structs/S_InventorySlots` _output_iteminfo _output_itemmesh (- _output_amount (`local.LocalAmount`))))
        (`self.UpdateSlotAtIndex` (`local.LocalIndex`))
        (return true)))
    (else
      (return false))))

(fn `SearchEmptySlot`
  (params (ItemType :type "/Game/GameFiles/Interactables/Enums/E_ItemTypeEnum Enum" :default "NewEnumerator8"))
  (returns (Success :type Boolean) (Index :type Integer))
  (locals (`EmptySlot?` :type Boolean) (CurrentIndex :type Integer))
  (bind _inventoryslot (`self.GetItemSlot` ItemType))
  (for (_array_element _array_index) _inventoryslot
    (if (not (`KismetSystemLibrary.IsValid` (`.ItemMesh_17_ABCAB25E4B6C9235D6D6279073793DD2` (break `/Game/GameFiles/Interactables/Structs/S_InventorySlots` _array_element))))
      (set `local.EmptySlot?` true)
      (set `local.CurrentIndex` _array_index)
      (break)))
  (return (`local.EmptySlot?`) (`local.CurrentIndex`)))

(fn `SearchFreeStack`
  (params (ItemReference :type "/Game/GameFiles/Interactables/MasterBlueprints/BP_PickUpMaster Object Reference") (ItemType :type "/Game/GameFiles/Interactables/Enums/E_ItemTypeEnum Enum" :default "NewEnumerator8"))
  (returns (`Success?` :type Boolean) (Index :type Integer))
  (locals (`StackFull?` :type Boolean) (CurrentIndex :type Integer))
  (bind _inventoryslot (`self.GetItemSlot` ItemType))
  (for (_array_element _array_index) _inventoryslot
    (bind (_iteminfo _itemmesh _amount) (break `/Game/GameFiles/Interactables/Structs/S_InventorySlots` _array_element))
    (if (`KismetSystemLibrary.IsValid` _itemmesh)
      (if (and (`KismetTextLibrary.EqualEqual_TextText` (`.Name_2_370516F44D1CDDEAD8897AB54DA1646D` (break `/Game/GameFiles/Interactables/Structs/S_ItemStruct` (`/Game/GameFiles/Interactables/MasterBlueprints/BP_PickUpMaster.ItemInfo` ItemReference))) (`.Name_2_370516F44D1CDDEAD8897AB54DA1646D` (break `/Game/GameFiles/Interactables/Structs/S_ItemStruct` _iteminfo))) (< _amount (`self.MaxStackSize`)))
        (set `local.StackFull?` true)
        (set `local.CurrentIndex` _array_index)
        (break))))
  (return (`local.StackFull?`) (`local.CurrentIndex`)))

(fn `SetItemInSlot`
  (params (ItemType :type "/Game/GameFiles/Interactables/Enums/E_ItemTypeEnum Enum" :default "NewEnumerator8") (Index :type Integer) (ObjectReference :type "/Game/GameFiles/Interactables/MasterBlueprints/BP_PickUpMaster Object Reference") (Amount :type Integer))
  (locals (LocalIndex :type Integer) (LocalObjectReference :type "/Game/GameFiles/Interactables/MasterBlueprints/BP_PickUpMaster Object Reference") (LocalAmount :type Integer))
  (bind _localobjectreference (`local.LocalObjectReference`))
  (bind _localobjectreference_2 (`local.LocalObjectReference`))
  (bind _localobjectreference_3 (`local.LocalObjectReference`))
  (bind _localobjectreference_4 (`local.LocalObjectReference`))
  (set `local.LocalIndex` Index)
  (set `local.LocalObjectReference` ObjectReference)
  (set `local.LocalAmount` Amount)
  (switch `/Game/GameFiles/Interactables/Enums/E_ItemTypeEnum` ItemType
    (:`NewEnumerator8`
      (set `self.CurrentInventoryTab` "NewEnumerator8" :!label _label)
      (`KismetArrayLibrary.Array_Set` (`self.UseableItemSlots`) (`local.LocalIndex`) (make `/Game/GameFiles/Interactables/Structs/S_InventorySlots` (`/Game/GameFiles/Interactables/MasterBlueprints/BP_PickUpMaster.ItemInfo` _localobjectreference) (`/Game/GameFiles/Interactables/MasterBlueprints/BP_PickUpMaster.SpawnedItemMesh` _localobjectreference) (`local.LocalAmount`))))
    (:`NewEnumerator12`
      (goto _label))
    (:`NewEnumerator0`
      (set `self.CurrentInventoryTab` "NewEnumerator10" :!label _label_2)
      (`KismetArrayLibrary.Array_Set` (`self.ArmorItemSlots`) (`local.LocalIndex`) (make `/Game/GameFiles/Interactables/Structs/S_InventorySlots` (`/Game/GameFiles/Interactables/MasterBlueprints/BP_PickUpMaster.ItemInfo` _localobjectreference_2) (`/Game/GameFiles/Interactables/MasterBlueprints/BP_PickUpMaster.SpawnedItemMesh` _localobjectreference_2) (`local.LocalAmount`))))
    (:`NewEnumerator1`
      (goto _label_2))
    (:`NewEnumerator2`
      (goto _label_2))
    (:`NewEnumerator3`
      (goto _label_2))
    (:`NewEnumerator4`
      (goto _label_2))
    (:`NewEnumerator5`
      (goto _label_2))
    (:`NewEnumerator6`
      (goto _label_2))
    (:`NewEnumerator7`
      (goto _label_2))
    (:`NewEnumerator9`
      (set `self.CurrentInventoryTab` "NewEnumerator0")
      (`KismetArrayLibrary.Array_Set` (`self.QuestItemSlots`) (`local.LocalIndex`) (make `/Game/GameFiles/Interactables/Structs/S_InventorySlots` (`/Game/GameFiles/Interactables/MasterBlueprints/BP_PickUpMaster.ItemInfo` _localobjectreference_3) (`/Game/GameFiles/Interactables/MasterBlueprints/BP_PickUpMaster.SpawnedItemMesh` _localobjectreference_3) (`local.LocalAmount`))))
    (:`NewEnumerator10`
      (set `self.CurrentInventoryTab` "NewEnumerator1")
      (`KismetArrayLibrary.Array_Set` (`self.ReadablesItemSlots`) (`local.LocalIndex`) (make `/Game/GameFiles/Interactables/Structs/S_InventorySlots` (`/Game/GameFiles/Interactables/MasterBlueprints/BP_PickUpMaster.ItemInfo` _localobjectreference_4) (`/Game/GameFiles/Interactables/MasterBlueprints/BP_PickUpMaster.SpawnedItemMesh` _localobjectreference_4) (`local.LocalAmount`))))))

(fn `ShowInventory`
  (`Widget.SetVisibility` (`self.InventoryWidget`) "Visible")
  (set `self.IsVisible?` true)
  (`Widget.SetIsEnabled` (`self.InventoryWidget`) true)
  (return))

(fn `SplitStackToIndex`
  (params (FromIndex :type Integer) (ToIndex :type Integer) (Amount :type Integer))
  (returns (`Success?` :type Boolean))
  (return false))

(fn `SwapSlots`
  (params (Index1 :type Integer) (Index2 :type Integer))
  (returns (`Success?` :type Boolean))
  (locals (LocalIndex1 :type Integer) (LocalIndex2 :type Integer))
  (bind _returnvalue (`KismetArrayLibrary.Array_LastIndex` (`self.GetItemTab` (`self.CurrentInventoryTab`))))
  (set `local.LocalIndex1` Index1)
  (set `local.LocalIndex2` Index2)
  (if (or (> (`local.LocalIndex1`) _returnvalue) (> (`local.LocalIndex2`) _returnvalue))
    (return false)))

(fn `UserConstructionScript`)