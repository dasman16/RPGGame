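; Item spawner that scatters random pickups from its location when play begins, such as a loot burst.
; BeginPlay makes five attempts, each running cascading random rolls that either spawn nothing or pick from SpawnableItems, with a hammer as the rarest result.
; RandomShoot spawns the item with its class-default ItemInfo and given amount, then launches its mesh with a force at random yaw and raised pitch, relative to the Sphere's rotation.
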(event `self.ReceiveBeginPlay`
  (bind _returnvalue (`KismetMathLibrary.RandomIntegerInRange` 1 3))
  (bind _returnvalue_2 (* (`KismetMathLibrary.RandomFloat`) 100.0))
  (for _ (range 1 6)
    (if (< _returnvalue_2 50.0)
      (`KismetSystemLibrary.PrintString` (`KismetStringLibrary.Conv_DoubleToString` _returnvalue_2))
      (elif (< _returnvalue_2 65.0)
        (`self.RandomShoot` (`|GetArrayItem` (`self.SpawnableItems`) 1) _returnvalue)
        (elif (< _returnvalue_2 75.0)
          (`self.RandomShoot` (`|GetArrayItem` (`self.SpawnableItems`) 2) _returnvalue)
          (elif (< _returnvalue_2 85.0)
            (`self.RandomShoot` (`|GetArrayItem` (`self.SpawnableItems`) (`KismetMathLibrary.RandomIntegerInRange` 3 4)) _returnvalue)
            (elif (< _returnvalue_2 99.0)
              (`self.RandomShoot` (`|GetArrayItem` (`self.SpawnableItems`)) _returnvalue)
              (else
                (`KismetSystemLibrary.PrintString` "spawned hammer")
                (`self.RandomShoot` (`|GetArrayItem` (`self.SpawnableItems`) 5) 1)))))))))

(fn `RandomShoot`
  (params (ItemToSpawn :type "/Game/GameFiles/Interactables/MasterBlueprints/BP_PickUpMaster Class Reference") (Amount :type Integer))
  (bind _returnvalue (`SceneComponent.K2_GetComponentLocation` (`self.DefaultSceneRoot`)))
  (bind (_returnvalue_roll _returnvalue_pitch _returnvalue_yaw) (`KismetMathLibrary.BreakRotator` (`SceneComponent.K2_GetComponentRotation` (`self.Sphere`))))
  (bind _returnvalue_2 (`|SpawnActorFromClass` ItemToSpawn (`KismetMathLibrary.MakeTransform` _returnvalue (`KismetMathLibrary.MakeRotator` 0.0 0.0 (`KismetMathLibrary.RandomFloatInRange` -180.0 180.0))) "Undefined" "OverrideRootScale" null (defaults `/Game/GameFiles/Interactables/BP_SpawnItems` ItemToSpawn) Amount "NewEnumerator12" "NewEnumerator8" null))
  (`PrimitiveComponent.AddForce` (`/Game/GameFiles/Interactables/MasterBlueprints/BP_InteractableObjectBaseMaster.DefaultMesh` _returnvalue_2) (* (- (+ _returnvalue (* (`KismetMathLibrary.GetForwardVector` (`KismetMathLibrary.MakeRotator` _returnvalue_roll (+ _returnvalue_pitch (`KismetMathLibrary.RandomFloatInRange` 45.0 60.0)) (+ _returnvalue_yaw (`KismetMathLibrary.RandomFloatInRange` -180.0 180.0)))) 200.0)) _returnvalue) 10000.0) "None" false))

(fn `UserConstructionScript`)