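; Master spawn area that fills a box volume with random craftable pickups and tops it up after a respawn delay.
; SpawnItems drops actors at random box points, traces down and retries until hitting Landscape, then aligns them to the surface and enables physics.
; After each delay, SetActorsToSpawn extends the box's Z extent and counts overlapping BP_PickUpCraftableMaster actors, so only the shortfall to NumberToSpawn respawns.
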(event `self.ReceiveBeginPlay`
  (`self.SpawnItems`))

(event `self.ReceiveTick`
  (params (DeltaSeconds :type "Float (single-precision)"))
  (`KismetSystemLibrary.Delay` (`self.RespawnTime`))
  (`self.SetActorsToSpawn`)
  (`self.SpawnItems`))

(fn `SetActorsToSpawn`
  (locals (ActorBox :type "BoxComponent Object Reference"))
  (bind _box (`self.Box`))
  (bind (_boxextent_x _boxextent_y _boxextent_z) (`KismetMathLibrary.BreakVector` (`BoxComponent.BoxExtent` _box)))
  (set `local.ActorBox` _box)
  (`BoxComponent.SetBoxExtent` (`local.ActorBox`) (`KismetMathLibrary.MakeVector` _boxextent_x _boxextent_y (+ _boxextent_z 10000.0)) true)
  (bind _outactors (`GameplayStatics.GetAllActorsOfClass` "/Script/Engine.Actor"))
  (for _array_element _outactors
    (bind _asbp_pick_up_craftable_master (cast `/Game/GameFiles/Interactables/MasterBlueprints/BP_PickUpCraftableMaster` _array_element))
    (if (`PrimitiveComponent.IsOverlappingActor` (`local.ActorBox`) _asbp_pick_up_craftable_master)
      (`/Engine/EditorBlueprintResources/StandardMacros.IncrementInt` (`self.NumberSpawned`)))))

(fn `SpawnActor`
  (locals (SpawnedObject :type "/Game/GameFiles/Interactables/MasterBlueprints/BP_PickUpCraftableMaster Object Reference"))
  (bind _box (`self.Box`))
  (bind _returnvalue (`|SpawnActorFromClass` (`|GetArrayItem` (`self.SpawnCraftables`) (`KismetMathLibrary.RandomInteger` 4)) (`KismetMathLibrary.MakeTransform` (`KismetMathLibrary.RandomPointInBoundingBox` (`SceneComponent.K2_GetComponentLocation` _box) (`BoxComponent.BoxExtent` _box))) "AdjustIfPossibleButDontSpawnIfColliding" "OverrideRootScale" null "NewEnumerator8" (struct) "NewEnumerator8" null :!label _label))
  (bind _output_get (set `local.SpawnedObject` _returnvalue))
  (set `self.ActorsToIgnore` (`|MakeArray` _returnvalue :!type "Actor Object Reference"))
  (bind (_returnvalue_x _returnvalue_y _returnvalue_z) (`KismetMathLibrary.BreakVector` (`SceneComponent.K2_GetComponentLocation` (`Actor.RootComponent` _output_get))))
  (bind _outhit (`KismetSystemLibrary.LineTraceSingle` (`KismetMathLibrary.MakeVector` _returnvalue_x _returnvalue_y _returnvalue_z) (`KismetMathLibrary.MakeVector` _returnvalue_x _returnvalue_y -20000.0) "TraceTypeQuery1" false (`self.ActorsToIgnore`)))
  (bind (_bblockinghit _binitialoverlap _time _distance _location _impactpoint _normal _impactnormal _physmat _hitactor) (`GameplayStatics.BreakHitResult` _outhit))
  (cast `Landscape` _hitactor
    (:`then`
      (`SceneComponent.K2_SetWorldLocationAndRotation` (`Actor.RootComponent` (`local.SpawnedObject`)) _impactpoint (`KismetMathLibrary.MakeRotFromZX` _impactnormal (`self.GetActorForwardVector`)) false true)
      (`/Engine/EditorBlueprintResources/StandardMacros.IncrementInt` (`self.NumberSpawned`)
        (:`  `
          (`PrimitiveComponent.SetSimulatePhysics` (`/Game/GameFiles/Interactables/MasterBlueprints/BP_InteractableObjectBaseMaster.DefaultMesh` (`local.SpawnedObject`)) true))))
    (:`CastFailed`
      (`self.K2_DestroyActor` (`local.SpawnedObject`))
      (goto _label))))

(fn `SpawnItems`
  (locals (SpawnedObject :type "/Game/GameFiles/Interactables/MasterBlueprints/BP_PickUpCraftableMaster Object Reference"))
  (for _ (range (`self.NumberSpawned`) (`self.NumberToSpawn`))
    (`self.SpawnActor`))
  (set `self.NumberSpawned` 0))

(fn `UserConstructionScript`)