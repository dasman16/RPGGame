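; BP_ArmorMaster is a master Blueprint for armor items that carry Stamina, Attack and Defence stats.
; SetArmorStats stores the three values, and SetArmorStatus compares them to pick an ArmorType for all zero, all at Max, all equal, tied highest pairs or a single highest stat.
; SetArmorName runs that classification, then appends the type's enum string to the name in ItemInfo.
; BeginPlay and construction only call the parent.
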(event `self.ReceiveBeginPlay`
  (`parent.ReceiveBeginPlay`))

(fn `SetArmorName`
  (bind (_iteminfo_name _iteminfo_icon _iteminfo_itemtype _iteminfo_canbestacked_ _iteminfo_canbeused_) (break `/Game/GameFiles/Interactables/Structs/S_ItemStruct` (`self.ItemInfo`)))
  (`self.SetArmorStatus`)
  (set `self.ItemInfo` (make `/Game/GameFiles/Interactables/Structs/S_ItemStruct` (`KismetTextLibrary.Conv_StringToText` (`KismetStringLibrary.Concat_StrStr` (`KismetTextLibrary.Conv_TextToString` _iteminfo_name) (`|GetEnumeratorNameAsString` (`self.ArmorType`)))) _iteminfo_icon _iteminfo_itemtype _iteminfo_canbestacked_ _iteminfo_canbeused_)))

(fn `SetArmorStats`
  (params (Stamina :type Integer) (Attack :type Integer) (Defence :type Integer))
  (set `self.Stamina` Stamina)
  (set `self.Attack` Attack)
  (set `self.Defence` Defence))

(fn `SetArmorStatus`
  (bind _stamina (`self.Stamina`))
  (bind _defence (`self.Defence`))
  (bind _defence_2 (`self.Defence`))
  (bind _attack (`self.Attack`))
  (bind _attack_2 (`self.Attack`))
  (bind _defence_3 (`self.Defence`))
  (bind _defence_4 (`self.Defence`))
  (bind _stamina_2 (`self.Stamina`))
  (bind _attack_3 (`self.Attack`))
  (bind _returnvalue (and (== _stamina _attack_2) (== _attack_2 _defence_4)))
  (if (and (== 0 _stamina) _returnvalue)
    (set `self.ArmorType` "NewEnumerator8")
    (elif (and _returnvalue (== _defence_4 (`self.Max`)))
      (set `self.ArmorType` "NewEnumerator0")
      (elif _returnvalue
        (set `self.ArmorType` "NewEnumerator12")
        (elif (and (== (`self.Attack`) _defence_2) (> _defence_2 (`self.Stamina`)))
          (set `self.ArmorType` "NewEnumerator13")
          (elif (and (== (`self.Stamina`) _attack_3) (> _attack_3 (`self.Defence`)))
            (set `self.ArmorType` "NewEnumerator14")
            (elif (and (== (`self.Stamina`) _defence) (> _defence (`self.Attack`)))
              (set `self.ArmorType` "NewEnumerator15")
              (elif (and (> _attack (`self.Defence`)) (> _attack (`self.Stamina`)))
                (set `self.ArmorType` "NewEnumerator1")
                (elif (and (> _defence_3 (`self.Attack`)) (> _defence_3 (`self.Stamina`)))
                  (set `self.ArmorType` "NewEnumerator2")
                  (elif (and (> _stamina_2 (`self.Defence`)) (> _stamina_2 (`self.Attack`)))
                    (set `self.ArmorType` "NewEnumerator3")))))))))))

(fn `UserConstructionScript`
  (`parent.UserConstructionScript`))